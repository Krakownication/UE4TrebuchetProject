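; Base physics gnome projectile that, once fired by a launcher, takes the camera and tracks flight distance and score.
; Tick updates the HUD, zeroes X velocity and detects stopping, then checks landing, notifies the launcher and teleports the mesh aside.
; Hit checks award door, pool and springboard bonuses, damping or boosting velocity, alongside height and upright-landing bonuses.
; Pressing R notifies the launcher and destroys the gnome.
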(event OnComponentHit(GnomeMesh)
  (params (HitComponent :type Primitive%20Component%20Object%20Reference) (OtherActor :type Actor%20Object%20Reference) (OtherComp :type Primitive%20Component%20Object%20Reference) (NormalImpulse :type Vector :default "0, 0, 0") (Hit :type Hit%20Result%20Structure%20%28by%20ref%29))
  ;[1 1 1] Hit Handlers
  (bind ___ (CallFunction|CheckDoorBonus OtherActor))
  (bind ____2 (CallFunction|CheckPoolBonus ___))
  (CallFunction|CheckSpringBoardBonus ____2))

(event EventTick
  (params (DeltaSeconds :type Float%20%28single-precision%29))
  (bind _hudconnector (Variables|Default|GetHUDConnector))
  (bind _gnomemesh (Variables|Default|GetGnomeMesh))
  (bind _gnomemesh_2 (Variables|Default|GetGnomeMesh))
  (bind _returnvalue (Transformation|GetComponentVelocity _gnomemesh))
  (bind _returnvalue_2 (Transformation|GetWorldTransform _gnomemesh_2))
  (if (not (Variables|Default|GetIsStopped))
    (if (Variables|Default|GetIsFired)
      ;[1 1 1] Calc length+score and send HUD updates
      (bind _currentlength (CallFunction|CalculateCurrentLength))
      (bind _currentscore (CallFunction|CalculateCurrentScore (- _currentlength (Variables|Default|GetCurrentLength))))
      (Variables|Default|SetCurrentScore _currentscore)
      (bind _output_get (Variables|Default|SetCurrentLength _currentlength))
      (Default|UpdateHUDLength _hudconnector _output_get)
      (Default|UpdateHUDScore _hudconnector (Variables|Default|GetCurrentScore))
      (CallFunction|CheckHeightBonus)
      (if (Math|Float|NearlyEqual(Float) (.x _returnvalue) 0.0 0.0001)
        _
        (else
          ;[1 1 1] Reset X Velocity
          (Physics|SetPhysicsLinearVelocity (Variables|Default|GetGnomeMesh) (Math|Vector|MakeVector 0.0 (.y _returnvalue) (.z _returnvalue)) false "None")))
      ;[1 1 1] Check IsStopped
      (if (<= (Math|Vector|VectorLength (Transformation|GetComponentVelocity (Variables|Default|GetGnomeMesh))) 0.5)
        (Variables|Default|SetIsStopped true)
        ;[1 1 1] Stop Handle
        (Default|UpdateHUDProjectileStopped (Variables|Default|GetHUDConnector))
        (Input|DisableInput (Game|GetPlayerController 0))
        (Utilities|FlowControl|Delay 0.5)
        (bind _hasperfectlanded (CallFunction|CheckLandingStyle))
        (if _hasperfectlanded
          (Utilities|FlowControl|Delay 3.5)
          (else
            (Utilities|FlowControl|Delay 1.0)))
        (Class|ILuncher|ProjectileStopped(Message) (Variables|Default|GetLuncher))
        (Transformation|SetWorldTransform (Variables|Default|GetGnomeMesh) (Math|Transform|MakeTransform (Math|Vector|MakeVector (+ (.x (.location _returnvalue_2)) -5e+02 (Math|Conversions|ToFloat(Integer) (Math|Random|RandomIntegerinRange -100 100))) (.y (.location _returnvalue_2)) 1.5e+02) "0, 0, 0" "1,1,1") false true)
        (Default|UpdateHUDLunchSetup (Variables|Default|GetHUDConnector))))))

(event EventLunch
  (params (Launcher :type Actor%20Object%20Reference%20%28by%20ref%29))
  (bind _returnvalue (Game|GetPlayerController 0))
  ;[1 1 1] Lunch Setup
  (Variables|Default|SetLuncher Launcher)
  (Variables|Default|SetIsFired true)
  (Variables|Default|SetStartLocation (Transformation|GetWorldLocation (Variables|Default|GetGnomeMesh)))
  (Input|EnableInput _returnvalue)
  (Game|Player|SetViewTargetwithBlend _returnvalue self 0.0 "VTBlend_Linear" 0.0 false)
  (Default|UpdateHUDLaunched (Variables|Default|GetHUDConnector)))

(event EventSetConnector
  (params (HUDConnector :type HUD%20Connector%20Object%20Reference%20%28by%20ref%29))
  (Variables|Default|SetHUDConnector HUDConnector))

(event Input|KeyboardEvents|R
  (params (Key :type Key%20Structure))
  ;[1 1 1] Restart Handler
  (:Pressed
    (Class|ILuncher|ProjectileStopped(Message) (Variables|Default|GetLuncher))
    (Actor|DestroyActor)))

(fn ConstructionScript)

(fn CalculateCurrentLength
  (bind _gnomemesh (Variables|Default|GetGnomeMesh))
  (bind _startlocation (Variables|Default|GetStartLocation))
  (bind _returnvalue (Transformation|GetWorldLocation _gnomemesh))
  (bind _returnvalue_2 (- _returnvalue _startlocation))
  (bind _returnvalue_3 (Math|Vector|VectorLength _returnvalue_2))
  (bind _returnvalue_4 (/ _returnvalue_3 1e+02))
  (bind _returnvalue_5 (Math|Float|Round _returnvalue_4))
  (if (< (.Y (Math|Vector|BreakVector _returnvalue)) (.Y (Math|Vector|BreakVector _startlocation)))
    (return _returnvalue_5)
    (else
      (return (* _returnvalue_5 -1)))))

(fn CalculateCurrentScore
  (params (DeltaLength :type Integer))
  (return (+ (Variables|Default|GetCurrentScore) (* DeltaLength 50) (Math|Float|Truncate (* (Math|Vector|VectorLength (Transformation|GetComponentVelocity (Variables|Default|GetGnomeMesh))) 0.005)))))

(fn CheckLandingStyle
  (bind _gnomemesh (Variables|Default|GetGnomeMesh))
  (bind _perfectlandingbonusangletolerance (LocalVariables|GetPerfectLandingBonusAngleTolerance))
  (bind _returnvalue (Transformation|GetWorldRotation _gnomemesh))
  (if (and (Math|Float|NearlyEqual(Float) (.roll _returnvalue) 0.0 _perfectlandingbonusangletolerance) (Math|Float|NearlyEqual(Float) (.pitch _returnvalue) 0.0 _perfectlandingbonusangletolerance))
    (CallFunction|ApplyBonus (LocalVariables|GetPerfectLandingBonusValue) (LocalVariables|GetPerfectLandingBonusText))
    (return true)
    (else
      (return false))))

(fn CheckHeightBonus
  (if (not (Variables|Default|GetHasHeightBonus))
    (if (>= (.z (Transformation|GetWorldLocation (Variables|Default|GetGnomeMesh))) (Math|Conversions|ToFloat(Integer) (LocalVariables|GetHighFlyThreshold)))
      (Variables|Default|SetHasHeightBonus true)
      (CallFunction|ApplyBonus (LocalVariables|GetHighFlyBonusValue) (LocalVariables|GetHighFlyBonusText)))))

(fn CheckDoorBonus
  (params (OverlappedActor :type Actor%20Object%20Reference))
  (if (Utilities|ClassIsChildOf (Utilities|GetClass OverlappedActor) "/Game/BProjectBP/Blueprints/Obstacles/Gate.Gate_C")
    (if (Variables|Default|GetHasDoorBonus)
      _
      (else
        (Variables|Default|SetHasDoorBonus true)
        (CallFunction|ApplyBonus (LocalVariables|GetDoorBonusValue) (LocalVariables|GetDoorBonusText))
        (return true OverlappedActor))))
  (return false OverlappedActor))

(fn CheckPoolBonus
  (params (OverlappedActor :type Actor%20Object%20Reference))
  (bind _gnomemesh (Variables|Default|GetGnomeMesh))
  (if (Utilities|ClassIsChildOf (Utilities|GetClass OverlappedActor) "/Game/BProjectBP/Blueprints/Obstacles/Pool.Pool_C")
    (if (Variables|Default|GetHasPoolBonus)
      _
      (else
        (Variables|Default|SetHasPoolBonus true)
        (Physics|SetPhysicsLinearVelocity _gnomemesh (* (Transformation|GetComponentVelocity _gnomemesh) 0.1) false "None")
        (CallFunction|ApplyBonus (LocalVariables|GetPoolBonusValue) (LocalVariables|GetPoolBonusText))
        (return true OverlappedActor))))
  (return false OverlappedActor))

(fn ApplyBonus
  (params (BonusValue :type Integer) (BonusText :type String))
  (bind _hudconnector (Variables|Default|GetHUDConnector))
  (bind _output_get (Variables|Default|SetCurrentScore (+ (Variables|Default|GetCurrentScore) BonusValue)))
  (Default|UpdateHUDScore _hudconnector _output_get)
  (Default|UpdateHUDNewBonus _hudconnector (Utilities|String|BuildString(Integer) BonusText " +" BonusValue)))

(fn CheckSpringBoardBonus
  (params (OverlappedActor :type Actor%20Object%20Reference))
  (bind _gnomemesh (Variables|Default|GetGnomeMesh))
  (bind _returnvalue (Transformation|GetComponentVelocity _gnomemesh))
  (if (Utilities|ClassIsChildOf (Utilities|GetClass OverlappedActor) "/Game/BProjectBP/Blueprints/Obstacles/SpringBoard.SpringBoard_C")
    (if (Variables|Default|GetIsSpringBoardBonusEnabled)
      (if (> (Math|Vector|VectorLength (Transformation|GetComponentVelocity _gnomemesh)) 6e+02)
        (if (>= (.z _returnvalue) 1.5e+02)
          (Variables|Default|SetIsSpringBoardBonusEnabled false)
          (Physics|SetPhysicsLinearVelocity _gnomemesh (Math|Vector|MakeVector 0.0 (- (* -1 (Math|Float|Absolute(Float) (.y _returnvalue))) 1e+03) (+ (* (Math|Float|Absolute(Float) (.z _returnvalue)) 1.25) 1e+03)) false "None")
          (Utilities|Time|SetTimerbyFunctionName 0 "EnableSpringBoardBonus" 1.0)
          (CallFunction|ApplyBonus (LocalVariables|GetSpringBoardBonusValue) (LocalVariables|GetSpringBoardBonusText))
          (return true OverlappedActor)
          (else
            _)))))
  (return false OverlappedActor))

(fn EnableSpringBoardBonus
  (Variables|Default|SetIsSpringBoardBonusEnabled true))