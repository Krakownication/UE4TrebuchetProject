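; Fat gnome Blueprint, a launchable gnome variant whose skill drives it sharply downward.
; It extends the parent's Lunch event to show the skill name on the HUD.
; Space Bar, handled directly here pending a parent event dispatcher, applies a large downward impulse to the gnome mesh.
; A flag and timer enforce the cooldown, which is also sent to the HUD on activation.
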(event EventLunch
  (params (Launcher :type Actor%20Object%20Reference%20%28by%20ref%29))
  (|CallParentFunction Launcher)
  (Default|UpdateHUDSetSkillName (Variables|Default|GetHUDConnector) (Variables|Default|GetSkillName)))

(event Input|KeyboardEvents|SpaceBar
  (params (Key :type Key%20Structure))
  ;[1 1 1] Handle Activate Skill | Todo: Event Dispatcher'a z poziomu parenta
  (:Pressed
    (if (not (Variables|Default|GetIsSkillOnCooldown))
      (Variables|Default|SetIsSkillOnCooldown true)
      (Utilities|Time|SetTimerbyFunctionName 0 "ResetSkillCooldown" (Variables|Default|GetSkillCooldown))
      (Physics|AddImpulse (Variables|Default|GetGnomeMesh) "0, 0,-40000.000000" "None" false)
      (Default|UpdateHUDSkilActivated (Variables|Default|GetHUDConnector) (Variables|Default|GetSkillCooldown)))))

(fn ConstructionScript)

(fn ResetSkillCooldown
  (Variables|Default|SetIsSkillOnCooldown false))