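; Tall gnome variant of a launchable gnome Blueprint, adding a SpaceBar skill with a cooldown.
; On launch it runs the parent logic and sends the skill name to the HUD connector.
; The skill snaps the mesh to a fixed rotation, zeroes its spin and applies a strong impulse along world negative Y.
; A timer clears the cooldown flag, while the HUD receives the cooldown duration.
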(event EventLunch
  (params (Launcher :type Actor%20Object%20Reference%20%28by%20ref%29))
  (|CallParentFunction Launcher)
  (Default|UpdateHUDSetSkillName (Variables|Default|GetHUDConnector) (Variables|Default|GetSkillName)))

(event Input|KeyboardEvents|SpaceBar
  (params (Key :type Key%20Structure))
  (bind _gnomemesh (Variables|Default|GetGnomeMesh))
  ;[1 1 1] Handle Activate Skill | Todo: Event Dispatcher'a z poziomu parenta
  (:Pressed
    (if (not (Variables|Default|GetIsSkillOnCooldown))
      (Variables|Default|SetIsSkillOnCooldown true)
      (Utilities|Time|SetTimerbyFunctionName 0 "ResetSkillCooldown" (Variables|Default|GetSkillCooldown))
      (Transformation|SetWorldRotation _gnomemesh "0, 0,-90.000000" false false)
      (Class|PrimitiveComponent|SetPhysicsAngularVelocityinRadians _gnomemesh "0, 0, 0" false "None")
      (Physics|AddImpulse _gnomemesh "0,-20000.000000,0.000000" "None" false)
      (Default|UpdateHUDSkilActivated (Variables|Default|GetHUDConnector) (Variables|Default|GetSkillCooldown)))))

(fn ConstructionScript)

(fn ResetSkillCooldown
  (Variables|Default|SetIsSkillOnCooldown false))