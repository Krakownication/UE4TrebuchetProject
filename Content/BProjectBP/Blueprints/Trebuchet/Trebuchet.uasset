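; Player-operated trebuchet that launches the selected gnome projectile and reports its stages to the HUD connector.
; One action input cycles arm, swing and release by rotating the LeverOperator, with IsPending blocking input mid-move.
; Arming spawns the gnome at the lever tip, binds the Rope constraint and Cable, then teleports it onto the base.
; Release detaches it, notifies it and disables input until ProjectileStopped restores input and view.
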(event EventBeginPlay
  (bind _returnvalue (Game|GetPlayerController 0))
  ;[1 1 1] Enable control
  (Utilities|FlowControl|Delay 1.0)
  (Input|EnableInput _returnvalue)
  (Game|Player|SetViewTargetwithBlend _returnvalue self 0.0 "VTBlend_Linear" 0.0 false)
  (Default|UpdateHUDLunchSetup (Variables|Default|GetHUDConnector)))

(event EventProjectileStopped
  (bind _returnvalue (Game|GetPlayerController 0))
  ;[1 1 1] Enable control
  (Input|EnableInput _returnvalue)
  (Game|Player|SetViewTargetwithBlend _returnvalue self 0.0 "VTBlend_Linear" 0.0 false)
  (Default|UpdateHUDLunchSetup (Variables|Default|GetHUDConnector)))

(event EventSetProjectileType
  (params (ProjectileClass :type Gnome%20Base%20Class%20Reference))
  (Variables|Default|SetSelectedGnome ProjectileClass))

(event Input|ActionEvents|InputActionAction
  (params (Key :type Key%20Structure))
  (bind _leveroperator (Variables|Default|GetLeverOperator))
  (bind _leveroperator_2 (Variables|Default|GetLeverOperator))
  ;[1 1 1] Input Handler
  (:Pressed
    (if (not (Variables|Default|GetIsPending))
      (if (Variables|Default|GetIsArmed)
        ;;[1 1 1] Start Lunching
        (Default|UpdateHUDLunchStarted (Variables|Default|GetHUDConnector))
        (Variables|Default|SetIsPending true)
        (Components|MoveComponentTo _leveroperator (Variables|/Script/Engine.SceneComponent|GetRelativeLocation _leveroperator) "0, 0,-55.000000" true true 0.5 true)
        (Variables|Default|SetIsPending false)
        (Variables|Default|SetIsLunched true)
        (Variables|Default|SetIsArmed false)
        (elif (Variables|Default|GetIsLunched)
          (CallFunction|DetachProjectile)
          (Variables|Default|SetIsLunched false)
          (Input|DisableInput (Game|GetPlayerController 0))
          (else
            ;;[1 1 1] Start Arming
            (Variables|Default|SetIsPending true)
            (Default|UpdateHUDArmStarted (Variables|Default|GetHUDConnector))
            (Components|MoveComponentTo _leveroperator_2 (Variables|/Script/Engine.SceneComponent|GetRelativeLocation _leveroperator_2) "0, 0,120.000000" true true 2.0 true)
            (CallFunction|CreateandAttachProjectile)
            (Variables|Default|SetIsPending false)
            (Variables|Default|SetIsArmed true)))))))

(fn ConstructionScript)

(fn DetachProjectile
  (bind _cable (Variables|Default|GetCable))
  (Class|PhysicsConstraintComponent|BreakConstraint (Variables|Default|GetRope))
  (Variables|/Script/CableComponent.CableComponent|SetbAttachEnd _cable false)
  (Variables|/Script/CableComponent.CableComponent|SetbEnableCollision _cable true)
  (Transformation|DetachFromComponent (Variables|Default|GetProjectileComponent) "KeepWorld" "KeepWorld" "KeepWorld" true)
  (Class|IProjectile|Lunch(Message) (Variables|/Script/Engine.ChildActorComponent|GetChildActor (Variables|Default|GetProjectileComponent)) self)
  (return))

(fn CreateandAttachProjectile
  (bind _cable (Variables|Default|GetCable))
  ;[1 1 1] Spawn Projectile at current Lever's end position (for proper Physics Constrain attach)
  (bind _returnvalue (AddComponent|AddChildActorComponent false (Math|Transform|MakeTransform (Math|Transform|InverseTransformLocation (Transformation|GetActorTransform) (Math|Transform|TransformLocation (Transformation|GetWorldTransform (Variables|Default|GetLever)) "0, 0,530.000000")) "0, 0, 0" "1,1,1")))
  (ChildActorComponent|SetChildActorClass _returnvalue (Variables|Default|GetSelectedGnome))
  (Variables|Default|SetProjectileComponent _returnvalue)
  (Class|IHUDConnected|SetConnector(Message) (Variables|/Script/Engine.ChildActorComponent|GetChildActor _returnvalue) (Variables|Default|GetHUDConnector))
  ;[1 1 1] Set Physics Constrain
  (bind _asprimitive_component (Utilities|Casting|CastToPrimitiveComponent (Variables|/Script/Engine.Actor|GetRootComponent (Variables|/Script/Engine.ChildActorComponent|GetChildActor _returnvalue))))
  (Class|PhysicsConstraintComponent|SetConstrainedComponents (Variables|Default|GetRope) (Variables|Default|GetLever) "None" _asprimitive_component "None")
  ;[1 1 1] Attach Cable to Projectile
  (Class|CableComponent|SetAttachEndto _cable (Variables|/Script/Engine.ChildActorComponent|GetChildActor (Variables|Default|GetProjectileComponent)) "None" "None")
  (Variables|/Script/CableComponent.CableComponent|SetbAttachEnd _cable true)
  (Variables|/Script/CableComponent.CableComponent|SetbEnableCollision _cable true)
  ;[1 1 1] Move Projectile to starting point
  (Transformation|SetWorldLocation (Variables|/Script/Engine.Actor|GetRootComponent (Variables|/Script/Engine.ChildActorComponent|GetChildActor (Variables|Default|GetProjectileComponent))) (Math|Transform|TransformLocation (Transformation|GetWorldTransform (Variables|Default|GetBase)) "0, 0,200.000000") false true)
  (return))