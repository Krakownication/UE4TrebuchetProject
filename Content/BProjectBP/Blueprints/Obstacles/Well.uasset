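; Well obstacle that launches any gnome entering its trigger box and awards it a bonus.
; On box overlap it checks for a GnomeBase, waits briefly, then teleports the gnome's mesh upward and adds an impulse to throw it up and along negative world Y.
; It then calls ApplyBonus on the gnome with the well's bonus value and text.
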(event OnComponentBeginOverlap(Box)
  (params (OverlappedComponent :type Primitive%20Component%20Object%20Reference) (OtherActor :type Actor%20Object%20Reference) (OtherComp :type Primitive%20Component%20Object%20Reference) (OtherBodyIndex :type Integer) (bFromSweep :type Boolean) (SweepResult :type Hit%20Result%20Structure%20%28by%20ref%29))
  (if (Utilities|ClassIsChildOf (Utilities|GetClass OtherActor) "/Game/BProjectBP/Blueprints/Gnomes/GnomeBase.GnomeBase_C")
    (bind _asgnome_base (Utilities|Casting|CastToGnomeBase OtherActor))
    (Utilities|FlowControl|Delay 0.25)
    (Transformation|SetWorldLocation (Variables|/Game/BProjectBP/Blueprints/Gnomes/GnomeBase.GnomeBase_C|GetGnomeMesh _asgnome_base) (+ (Transformation|GetWorldLocation (Variables|/Game/BProjectBP/Blueprints/Gnomes/GnomeBase.GnomeBase_C|GetGnomeMesh _asgnome_base)) "0, 0,150.000000") false true)
    (Physics|AddImpulse (Variables|/Game/BProjectBP/Blueprints/Gnomes/GnomeBase.GnomeBase_C|GetGnomeMesh _asgnome_base) "0,-30000.000000,30000.000000" "None" false)
    (Default|ApplyBonus _asgnome_base (Variables|Bonus|GetWellBonusValue) (Variables|Bonus|GetWellBonusText))))

(event EventBeginPlay)

(event Collision|EventActorBeginOverlap
  (params (OtherActor :type Actor%20Object%20Reference)))

(event EventTick
  (params (DeltaSeconds :type Float%20%28single-precision%29)))

(fn ConstructionScript)